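; Checkpoint beacon that lights up when an actor implementing PlayerInterface enters its sphere.
; The overlap calls HandleGlowEffects, which is not defined in this graph, and sets the Reached flag.
; The CheckPointReached event receives a dynamic material instance and plays a timeline that drives its Glow parameter, scaled by GlowFactor.
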(event OnComponentBeginOverlap(Sphere)
  (params (OverlappedComponent :type Primitive%20Component%20Object%20Reference) (OtherActor :type Actor%20Object%20Reference) (OtherComp :type Primitive%20Component%20Object%20Reference) (OtherBodyIndex :type Integer) (bFromSweep :type Boolean) (SweepResult :type Hit%20Result%20Structure%20%28by%20ref%29))
  (if (Utilities|DoesObjectImplementInterface OtherActor "/Script/TestProject_Aura.PlayerInterface")
    (Class|CheckPoint|HandleGlowEffects)
    (Variables|Default|SetbReached true)))

(event EventCheckPointReached
  (params (DynamicMaterialInstance :type Material%20Instance%20Dynamic%20Object%20Reference))
  (bind _glow_track (Timeline|Beacon%20Timeline Play)
    (:Update
      (Rendering|Material|SetScalarParameterValue DynamicMaterialInstance "Glow" (* _glow_track (Variables|Default|GetGlowFactor)) :!class /Script/Engine.MaterialInstanceDynamic))))

(fn ConstructionScript)