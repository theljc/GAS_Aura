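; Gameplay ability for the goblin spear melee attack, damaging live actors around the weapon hit point.
; On activation it faces the combat target through CombatInterface, plays a random attack montage and waits for a montage-tag gameplay event.
; The event triggers a small sphere query at that tag's socket, ignoring the avatar, damages each result and ends the ability.
; Montage, event tag and socket tag each use a separately evaluated random index.
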(event Ability|EventActivateAbility
  (bind _returnvalue (Ability|GetAvatarActorfromActorInfo))
  (bind _returnvalue_2 (Ability|GetAvatarActorfromActorInfo))
  (bind _returnvalue_3 (Class|EnemyInterface|GetCombatTarget(Message) _returnvalue))
  (bind _ascombat_interface (Utilities|Casting|CastToCombatInterface _returnvalue))
  ;[1 1 1] 每次攻击时朝向目标
  (Class|CombatInterface|UpdateFacingTarget _ascombat_interface (Transformation|GetActorLocation _returnvalue_3))
  ;[1 1 1] 从所有结构体数据中随机取一个
  (bind _returnvalue_4 (Class|CombatInterface|GetAttackMontages(Message) (Ability|GetAvatarActorfromActorInfo)))
  (|PlayMontageandWaitProxy "None" (.Montage (Utilities|Struct|BreakTaggedMontage (Utilities|Array|Get(acopy) _returnvalue_4 (Math|Random|RandomIntegerinRange 0 (- (Utilities|Array|Length _returnvalue_4) 1))))) 1.0 "None" true 1.0 0.0 false
    (:then
      ;[1 1 1] 等待蒙太奇中的 Tag 事件
      (Ability|Tasks|WaitGameplayEvent (.MontageTag (Utilities|Struct|BreakTaggedMontage (Utilities|Array|Get(acopy) _returnvalue_4 (Math|Random|RandomIntegerinRange 0 (- (Utilities|Array|Length _returnvalue_4) 1))))) 0
        (:EventReceived
          ;[1 1 1] 获得插槽的位置进行球体检测
          (bind _returnvalue_5 (Class|CombatInterface|GetCombatSocketLocation(Message) _returnvalue_2 (.MontageTag (Utilities|Struct|BreakTaggedMontage (Utilities|Array|Get(acopy) _returnvalue_4 (Math|Random|RandomIntegerinRange 0 (- (Utilities|Array|Length _returnvalue_4) 1)))))))
          (bind _outoverlappingactors (Class|AuraAbilitySystemLibrary|GetLiveActorsWithinRadius _returnvalue_2 (Utilities|Array|MakeArray _returnvalue_2) 45.0 _returnvalue_5))
          (for _array_element _outoverlappingactors
            ;[1 1 1] 对检测到的所有 Actor（有 ASC 组件的 Actor）造成伤害
            (Class|AuraDamageGameplayAbility|CauseDamage _array_element))
          (Ability|EndAbility))))))

(event Ability|EventOnEndAbility
  (params (bWasCancelled :type Boolean)))