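; Arcane Shard gameplay ability that shows a magic circle, then plays shard effects at ground points around the location under the mouse once input is pressed.
; A spawned BP_PointCollection supplies the points with random yaw while the avatar turns to the target and plays the cast montage.
; The montage event hides the circle and starts a looping timer that fires one GameplayCue per point, then destroys the collection and ends the ability.
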(event Custom|Spawn%20Shard
  (if (< (Variables|Default|GetCount) (Variables|Default|GetNum%20Points))
    (Variables|Default|SetSpawn%20Location (Transformation|GetWorldLocation (Utilities|Array|Get(acopy) (Variables|Default|GetGroundPoints) (Variables|Default|GetCount))))
    (Math|Integer|IncrementInt (Variables|Default|GetCount)
      (:%20%20
        (Class|GameplayAbility|ExecuteGameplayCuewithParams "(TagName=\"GameplayCue.ArcaneShard\")" (Ability|GameplayCue|MakeGameplayCueParameters :Location (Variables|Default|GetSpawn%20Location)))))
    (else
      (Utilities|Time|ClearandInvalidateTimerbyHandle (Variables|Default|GetTimer%20Handle))
      (Utilities|FlowControl|Delay 0.2)
      (Actor|DestroyActor (Variables|Default|GetPointCollection))
      (Ability|EndAbility))))

(event Ability|EventActivateAbility
  (Utilities|FlowControl|Sequence
    (:then_0
      (Class|PlayerInterface|ShowMagicCircle(Message) (Ability|GetAvatarActorfromActorInfo) 0))
    (:then_1
      (Ability|Tasks|WaitInputPress false
        (:OnPress
          (bind _datahandle (|TargetDataUnderMouse)
            (:ValidData
              (bind _output_get (Variables|Default|SetMouse%20HIt%20Location (.ImpactPoint (Collision|BreakHitResult (Ability|TargetData|GetHitResultfromTargetData _datahandle)))))
              (bind _returnvalue (Game|SpawnActorfromClass "/Game/Blueprint/AbilitySystem/Aura/GA/Arcane/BP_PointCollection.BP_PointCollection_C" (Math|Transform|MakeTransform _output_get "0, 0, 0" "1.000000,1.000000,1.000000") "Undefined" "MultiplyWithRoot" 0 0))
              (bind _output_get_2 (Variables|Default|SetPointCollection _returnvalue))
              (Variables|Default|SetGroundPoints (Class|PointCollection|GetGroundPoints _output_get_2 (Variables|Default|GetMouse%20HIt%20Location) (Variables|Default|GetNum%20Points) (Math|Random|RandomFloatinRange 0.0 3.6e+02)))
              (Class|CombatInterface|UpdateFacingTarget(Message) (Ability|GetAvatarActorfromActorInfo) (Variables|Default|GetMouse%20HIt%20Location))
              (|PlayMontageandWaitProxy "None" "/Game/Assets/Characters/Aura/Animations/Abilities/AM_Cast_ArcaneShards.AM_Cast_ArcaneShards" 1.0 "None" true 1.0 0.0 false
                (:then
                  (Ability|Tasks|WaitGameplayEvent "(TagName=\"Event.Montage.AranceShard\")" 0 true
                    (:EventReceived
                      (bind _returnvalue_2 (Utilities|Time|SetTimerbyEvent (delegate Custom|Spawn%20Shard) (Variables|Default|GetShard%20Spawn%20Delta%20Time) true))
                      (Variables|Default|SetTimer%20Handle _returnvalue_2)
                      (Class|PlayerInterface|HideMagicCircle(Message) (Ability|GetAvatarActorfromActorInfo))
                      (CallFunction|SpawnShard))))))))))))