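; Fire Blast fireball projectile that flies out like a boomerang and explodes on returning to its ReturnToActor.
; Server-driven timelines lerp it out to TravelDistance, then back toward that actor's live location.
; Within ExplodeDistance it calls OnHit, manually executes the FireBlast GameplayCue and destroys itself.
; The blast applies radial GAS damage to live actors except its owner, with 45-degree-pitched knockback and a death impulse.
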(event EventStartOutgoingTimeline
  (bind _returnvalue (Components|GetOwner))
  (bind _array (Utilities|Array|MakeArray _returnvalue))
  (Networking|SwitchHasAuthority
    (:Authority
      (Variables|Default|SetInit%20Location (Transformation|GetActorLocation))
      (Variables|Default|SetApex%20Location (+ (Variables|Default|GetInit%20Location) (* (Transformation|GetActorForwardVector) (Variables|Default|GetTravel%20Distance))))
      (bind _outgoing_track (Timeline|Outgoing%20Timeline Play)
        (:Update
          (Transformation|SetActorLocation (Math|Vector|Lerp(Vector) (Variables|Default|GetInit%20Location) (Variables|Default|GetApex%20Location) _outgoing_track) false false))
        (:Finished
          (bind _returning_track (Timeline|ReturningTimeline Play)
            (:Update
              (Transformation|SetActorLocation (Math|Vector|Lerp(Vector) (Variables|Default|GetApex%20Location) (Transformation|GetActorLocation (Variables|Default|GetReturnToActor)) _returning_track) false false)
              (if (CallFunction|IsWithinExplodeDistance)
                (Class|AuraProjectile|OnHit)
                ;[1 1 1] OnHit函数没执行GC，手动执行
                (GameplayCue|ExecuteGameplayCueOnActor(Burst) (Components|GetOwner) "(TagName=\"GameplayCue.FireBlast\")" (Ability|GameplayCue|MakeGameplayCueParameters :Location (Transformation|GetActorLocation)))
                (Class|AuraAbilitySystemLibrary|SetIsRadialDamageEffectParam (Variables|Default|GetDamageEffectParam) true (Variables|Default|GetRadialDamageInnerRadius) (Variables|Default|GetRadialDamageOuterRadius) (Transformation|GetActorLocation))
                (Utilities|Array|Add _array self)
                (bind _outoverlappingactors (Class|AuraAbilitySystemLibrary|GetLiveActorsWithinRadius self _array (Variables|Default|GetRadialDamageOuterRadius) (Transformation|GetActorLocation)))
                (for _array_element _outoverlappingactors
                  (Class|AuraAbilitySystemLibrary|SetTargetEffectParamsASC (Variables|Default|GetDamageEffectParam) (Ability|GetAbilitySystemComponent _array_element))
                  (Variables|Default|SetKnockbackDirection (- (Transformation|GetActorLocation _array_element) (Transformation|GetActorLocation)))
                  (Class|AuraAbilitySystemLibrary|SetKnockbackDirection (Variables|Default|GetDamageEffectParam) (CallFunction|OverrideKnockbackPitch) (Variables|Default|GetKnockbackMagnitude))
                  (Class|AuraAbilitySystemLibrary|SetDeathImpulseDirection (Variables|Default|GetDamageEffectParam) (Variables|Default|GetKnockbackDirection) (Variables|Default|GetDeathImpulseMagnitude))
                  (Class|AuraAbilitySystemLibrary|ApplyDamageEffect (Variables|Default|GetDamageEffectParam)))
                (Actor|DestroyActor)))))))))

(fn ConstructionScript)

(fn IsWithinExplodeDistance
  (return (< (Math|Vector|VectorLength (- (Transformation|GetActorLocation) (Transformation|GetActorLocation (Variables|Default|GetReturnToActor)))) (Variables|Default|GetExplodeDistance))))

(fn OverrideKnockbackPitch
  (bind _knockbackdirection (Variables|Default|GetKnockbackDirection))
  (bind _returnvalue (Math|Rotator|MakeRotfromX _knockbackdirection))
  (return (Math|Vector|GetForwardVector (Math|Rotator|MakeRotator (.roll _returnvalue) 45.0 (.yaw _returnvalue)))))