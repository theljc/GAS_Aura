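; BP_AuraMainMenu is the Aura main menu actor that starts the menu music and UI and animates a floating fireball effect.
; BeginPlay caches the Niagara component's location, plays the music, adds WBP_MainMenu to the viewport and switches to UI-only input with a visible cursor.
; Tick advances a timer that resets after about two pi, feeding an amplitude-scaled sine that bobs the effect vertically around its start point.
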(event EventBeginPlay
  (Variables|Default|SetFireball%20Init%20Location (Transformation|GetWorldLocation (Variables|Default|GetNiagara)))
  (bind _returnvalue (Audio|SpawnSound2D "/Game/Assets/Sounds/Music/Music_MainMenu.Music_MainMenu" 1.0 1.0 0.0 0))
  (Variables|Default|SetMainMenu%20Music _returnvalue)
  (bind _returnvalue_2 (UserInterface|CreateWidget "/Game/Blueprint/UI/MainMenu/WBP_MainMenu.WBP_MainMenu_C"))
  (UserInterface|Viewport|AddtoViewport _returnvalue_2 0)
  (Input|SetInputModeUIOnly (Game|GetPlayerController 0) _returnvalue_2 "DoNotLock" false)
  (Variables|/Script/Engine.PlayerController|SetbShowMouseCursor (Game|GetPlayerController 0) true))

(event EventTick
  (params (DeltaSeconds :type Float%20%28single-precision%29))
  (CallFunction|UpdateTime DeltaSeconds)
  (Transformation|SetWorldLocation (Variables|Default|GetNiagara) (+ (Variables|Default|GetFireball%20Init%20Location) (Math|Vector|MakeVector 0.0 0.0 (CallFunction|SinTime))) false false))

(fn ConstructionScript)

(fn UpdateTime
  (params (A :type Float%20%28double-precision%29))
  (bind _output_get (Variables|Default|SetTime (+ A (Variables|Default|GetTime))))
  (if (> _output_get 6.28315)
    (Variables|Default|SetTime 0.0)))

(fn SinTime
  (return (* (Math|Trig|Sin(Radians) (Variables|Default|GetTime)) (Variables|Default|GetAmplitude))))