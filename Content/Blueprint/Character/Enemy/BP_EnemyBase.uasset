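; BP_EnemyBase is a base enemy character Blueprint that handles debug highlighting and dissolve effects.
; While HighLight is set, Tick draws a debug capsule matching the collision capsule.
; StartDissolveTimeline and StartWeaponDissolveTimeline each receive a dynamic material instance and play separate timelines that drive its "Dissolve" scalar parameter.
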(event EventBeginPlay)

(event Collision|EventActorBeginOverlap
  (params (OtherActor :type Actor%20Object%20Reference)))

(event EventTick
  (params (DeltaSeconds :type Float%20%28single-precision%29))
  (bind _capsulecomponent (Variables|Default|GetCapsuleComponent))
  (if (Variables|Default|GetHighLight)
    (Rendering|Debug|DrawDebugCapsule (Transformation|GetWorldLocation _capsulecomponent) (Variables|/Script/Engine.CapsuleComponent|GetCapsuleHalfHeight _capsulecomponent) (Variables|/Script/Engine.CapsuleComponent|GetCapsuleRadius _capsulecomponent) "0, 0, 0" "(R=1.000000,G=0.000000,B=0.206622,A=1.000000)" 0.0 0.0)))

(event EventStartDissolveTimeline
  (params (DynamicMaterialInstance :type Material%20Instance%20Dynamic%20Object%20Reference))
  (bind _dissolvetrack (Timeline|Dissolve Play)
    (:Update
      (Rendering|Material|SetScalarParameterValue DynamicMaterialInstance "Dissolve" _dissolvetrack :!class /Script/Engine.MaterialInstanceDynamic))))

(event EventStartWeaponDissolveTimeline
  (params (DynamicMaterialInstance :type Material%20Instance%20Dynamic%20Object%20Reference))
  (bind _dissolvetrack (Timeline|WeaponDissolve Play)
    (:Update
      (Rendering|Material|SetScalarParameterValue DynamicMaterialInstance "Dissolve" _dissolvetrack :!class /Script/Engine.MaterialInstanceDynamic))))

(fn ConstructionScript)