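; Actor that fades its static mesh out and back in through material swaps and a timeline.
; The construction script caches the mesh's original materials and builds dynamic instances from the assigned fade materials.
; FadeOut applies those instances and plays the timeline driving their "Fade" parameter, while Fadein reverses it.
; A finish at Fade 1 or above restores the original materials; the Visibility collision toggles are unconnected.
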(event EventBeginPlay)

(event EventFadeOut
  (for (_array_element _array_index) (Variables|Default|GetDynamicMaterialsInstance)
    (Rendering|Material|SetMaterial (Variables|Default|GetStaticMesh) _array_index _array_element)
    (bind _fade (Timeline|Fade Play)
      (:Update
        (for _array_element_2 (Variables|Default|GetDynamicMaterialsInstance)
          (Rendering|Material|SetScalarParameterValue _array_element_2 "Fade" _fade :!class /Script/Engine.MaterialInstanceDynamic)))
      (:Finished
        (CallFunction|FadeFinished _fade)))))

(event EventFadein
  (bind _fade (Timeline|Fade Reverse)
    (:Update
      (for _array_element (Variables|Default|GetDynamicMaterialsInstance)
        (Rendering|Material|SetScalarParameterValue _array_element "Fade" _fade :!class /Script/Engine.MaterialInstanceDynamic)))
    (:Finished
      (CallFunction|FadeFinished _fade))))

(fn ConstructionScript
  (Utilities|Array|Clear (Variables|Default|GetDynamicMaterialsInstance))
  (Variables|Default|SetOriginalMaterials (Rendering|Material|GetMaterials (Variables|Default|GetStaticMesh)))
  (for _array_element (Variables|Default|GetFadeMaterialsInstance)
    (bind _returnvalue (Rendering|Material|CreateDynamicMaterialInstance _array_element "None" "None" :!class /Script/Engine.KismetMaterialLibrary))
    (Utilities|Array|AddUnique (Variables|Default|GetDynamicMaterialsInstance) _returnvalue)))

(fn ResetMaterial
  (for (_array_element _array_index) (Variables|Default|GetOriginalMaterials)
    (Rendering|Material|SetMaterial (Variables|Default|GetStaticMesh) _array_index _array_element)))

(fn FadeFinished
  (params (A :type Float%20%28double-precision%29))
  (if (>= A 1.0)
    (CallFunction|ResetMaterial)
    (elif (<= A 0.0)
      _)))